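; BPC_PositionRing is a component on BP_XRCharacter that displays a position ring where a vertical trace from the character hits a surface.
; Each tick it line-traces along Z by TraceLength from the actor location and stores whether it hit in BeneathBoard.
; On a hit it shows itself and passes the slightly raised impact location to the character's SetRingPosition; otherwise it hides and passes the actor location.
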(event `self.ReceiveBeginPlay`
  (bind _asbp_xrcharacter (cast `/Game/Blueprints/Characters/BP_XRCharacter` (`self.GetOwner`)))
  (set `self.As BP XRCharacter` _asbp_xrcharacter))

(event `self.ReceiveTick`
  (params (DeltaSeconds :type "Float (single-precision)"))
  (bind _as_bp_xrcharacter (`self.As BP XRCharacter`)
    (:`then`
      (bind _returnvalue (`Actor.K2_GetActorLocation` _as_bp_xrcharacter))
      (bind _outhit (`KismetSystemLibrary.LineTraceSingle` :`Start` _returnvalue :`End` (+ _returnvalue (`KismetMathLibrary.MakeVector` 0.0 0.0 (`self.traceLength`))) :`TraceChannel` "TraceTypeQuery4" :`DrawTime` 0.5))
      (bind _output_get (set `self.bBeneathBoard` (`GameplayStatics.BreakHitResult` _outhit)))
      (if _output_get
        (`self.SetVisibility` true)
        (`/Game/Blueprints/Characters/BP_XRCharacter.SetRingPosition` (`self.As BP XRCharacter`) (+ (`.Location` (`GameplayStatics.BreakHitResult` _outhit)) (0.0 0.0 0.5)))
        (else
          (`self.SetVisibility` false)
          (`/Game/Blueprints/Characters/BP_XRCharacter.SetRingPosition` (`self.As BP XRCharacter`) _returnvalue))))
    (:`else`)))