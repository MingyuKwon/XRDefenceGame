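; BP_XRGamePlayMode is the XR gameplay game mode, which locates the level's pool manager and shows a debug readout of it.
; A looping timer started on BeginPlay searches for a BP_PoolManager actor until one is found and cached, then keeps firing without searching.
; Once the manager is found, Tick prints its pool count for the OffenceT type to screen every frame.
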(event `self.ReceiveBeginPlay`
  (`KismetSystemLibrary.K2_SetTimerDelegate` (delegate `커스텀이벤트`) 0.2 true))

(event `커스텀이벤트`
  (if (not (`self.bPoolFind`))
    (bind _outactors (`GameplayStatics.GetAllActorsOfClass` "/Game/Blueprints/Manager/BP_PoolManager.BP_PoolManager_C"))
    (if (> (`KismetArrayLibrary.Array_Length` _outactors) 0)
      (set `self.PoolManager` (`|GetArrayItem` _outactors))
      (set `self.bPoolFind` true))))

(event `self.ReceiveTick`
  (params (DeltaSeconds :type "Float (single-precision)"))
  (if (`self.bPoolFind`)
    (bind _typecount (`/Game/Blueprints/Manager/BP_PoolManager.GetPoolCountOfType` (`self.PoolManager`) "ECT_OffenceT"))
    (`KismetSystemLibrary.PrintString` (`KismetStringLibrary.Conv_Int64ToString` _typecount) true true (struct :`R` 1.0 :`G` 0.022204 :`A` 1.0) -1.0 "-1")))

(fn `UserConstructionScript`)