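; Pool manager that hands out pre-existing offence units, gold mines and defence tower variants by character type.
; BeginPlay caches all level actors of each class into per-type arrays, which GetArrayClassFromEnum selects alongside a class from SpawnClassMap.
; PoolSpawnActor claims the first actor whose pool flag is set by clearing it, returning nothing if none is free rather than spawning.
; GetPoolCountOfType counts the actors still pooled for a type.
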(event `self.ReceiveBeginPlay`
  (`|ExecutionSequence`
    (:`then_0`
      (bind _outactors (`GameplayStatics.GetAllActorsOfClass` "/Game/Blueprints/Characters/Offence/BP_OffenceT.BP_OffenceT_C"))
      (set `self.OffenceTArray` _outactors)
      (bind _outactors_2 (`GameplayStatics.GetAllActorsOfClass` "/Game/Blueprints/Characters/Offence/BP_OffenceD.BP_OffenceD_C"))
      (set `self.OffenceDArray` _outactors_2))
    (:`then_1`
      (bind _outactors_3 (`GameplayStatics.GetAllActorsOfClass` "/Game/Blueprints/Characters/Offence/BP_OffenceDT.BP_OffenceDT_C"))
      (set `self.OffenceDTArray` _outactors_3)
      (bind _outactors_4 (`GameplayStatics.GetAllActorsOfClass` "/Game/Blueprints/Characters/Offence/BP_OffenceH.BP_OffenceH_C"))
      (set `self.OffenceHArray` _outactors_4))
    (:`then_2`
      (bind _outactors_5 (`GameplayStatics.GetAllActorsOfClass` "/Game/Blueprints/Characters/Offence/BP_OffenceS.BP_OffenceS_C"))
      (set `self.OffenceSArray` _outactors_5)
      (bind _outactors_6 (`GameplayStatics.GetAllActorsOfClass` "/Game/Blueprints/Characters/Offence/BP_OffenceB.BP_OffenceB_C"))
      (set `self.OffenceBArray` _outactors_6))
    (:`then_3`
      (bind _outactors_7 (`GameplayStatics.GetAllActorsOfClass` "/Game/Blueprints/Characters/BP_GoldMine.BP_GoldMine_C"))
      (set `self.GoldMineArray` _outactors_7)
      (bind _outactors_8 (`GameplayStatics.GetAllActorsOfClass` "/Game/Blueprints/Characters/Offence/BP_OffenceL.BP_OffenceL_C"))
      (set `self.OffenceLArray` _outactors_8))
    (:`then_4`
      (bind _outactors_9 (`GameplayStatics.GetAllActorsOfClass` "/Game/Blueprints/Characters/Defence/BP_DefenceT.BP_DefenceT_C"))
      (set `self.DefenceTArray` _outactors_9)
      (bind _outactors_10 (`GameplayStatics.GetAllActorsOfClass` "/Game/Blueprints/Characters/Defence/BP_DefenceT_Laser_1.BP_DefenceT_Laser_1_C"))
      (set `self.DefenceTL1Array` _outactors_10)
      (bind _outactors_11 (`GameplayStatics.GetAllActorsOfClass` "/Game/Blueprints/Characters/Defence/BP_DefenceT_Laser_2.BP_DefenceT_Laser_2_C"))
      (set `self.DefenceTL2Array` _outactors_11))
    (:`then_5`
      (bind _outactors_12 (`GameplayStatics.GetAllActorsOfClass` "/Game/Blueprints/Characters/Defence/BP_DefenceT_Canon_1.BP_DefenceT_Canon_1_C"))
      (set `self.DefenceTC1Array` _outactors_12)
      (bind _outactors_13 (`GameplayStatics.GetAllActorsOfClass` "/Game/Blueprints/Characters/Defence/BP_DefenceT_Canon_2.BP_DefenceT_Canon_2_C"))
      (set `self.DefenceTC2Array` _outactors_13))
    (:`then_6`
      (bind _outactors_14 (`GameplayStatics.GetAllActorsOfClass` "/Game/Blueprints/Characters/Defence/BP_DefenceT_Fire1.BP_DefenceT_Fire1_C"))
      (set `self.DefenceTF1Array` _outactors_14)
      (bind _outactors_15 (`GameplayStatics.GetAllActorsOfClass` "/Game/Blueprints/Characters/Defence/BP_DefenceT_Fire2.BP_DefenceT_Fire2_C"))
      (set `self.DefenceTF2Array` _outactors_15))
    (:`then_7`
      (bind _outactors_16 (`GameplayStatics.GetAllActorsOfClass` "/Game/Blueprints/Characters/Defence/BP_DefenceT_Arrow1.BP_DefenceT_Arrow1_C"))
      (set `self.DefenceTA1Array` _outactors_16)
      (bind _outactors_17 (`GameplayStatics.GetAllActorsOfClass` "/Game/Blueprints/Characters/Defence/BP_DefenceT_Arrow2.BP_DefenceT_Arrow2_C"))
      (set `self.DefenceTA2Array` _outactors_17))))

(fn `Get Array Class from Enum`
  (params (CharacterType :type "ECharacterType Enum" :default "ECT_OffenceD"))
  (returns (outClass :type "XR_Character Class Reference") (outArray :type "Array of XR_Character Object Reference"))
  (locals (OutTempArray :type "Array of XR_Character Object Reference"))
  (switch `ECharacterType` CharacterType
    (:`ECT_OffenceD`
      (set `local.OutTempArray` (`self.OffenceDArray`)))
    (:`ECT_OffenceDT`
      (set `local.OutTempArray` (`self.OffenceDTArray`)))
    (:`ECT_OffenceT`
      (set `local.OutTempArray` (`self.OffenceTArray`)))
    (:`ECT_OffenceH`
      (set `local.OutTempArray` (`self.OffenceHArray`)))
    (:`ECT_OffenceB`
      (set `local.OutTempArray` (`self.OffenceBArray`)))
    (:`ECT_OffenceS`
      (set `local.OutTempArray` (`self.OffenceSArray`)))
    (:`ECT_OffenceL`
      (set `local.OutTempArray` (`self.OffenceLArray`)))
    (:`ECT_Gold`
      (set `local.OutTempArray` (`self.GoldMineArray`)))
    (:`ECT_DefenceT`
      (set `local.OutTempArray` (`self.DefenceTArray`)))
    (:`ECT_DefenceT_Laser_1`
      (set `local.OutTempArray` (`self.DefenceTL1Array`)))
    (:`ECT_DefenceT_Laser_2`
      (set `local.OutTempArray` (`self.DefenceTL2Array`)))
    (:`ECT_DefenceT_Canon_1`
      (set `local.OutTempArray` (`self.DefenceTC1Array`)))
    (:`ECT_DefenceT_Canon_2`
      (set `local.OutTempArray` (`self.DefenceTC2Array`)))
    (:`ECT_DefenceT_Fire_1`
      (set `local.OutTempArray` (`self.DefenceTF1Array`)))
    (:`ECT_DefenceT_Fire_2`
      (set `local.OutTempArray` (`self.DefenceTF2Array`)))
    (:`ECT_DefenceT_Arrow_1`
      (set `local.OutTempArray` (`self.DefenceTA1Array`)))
    (:`ECT_DefenceT_Arrow_2`
      (set `local.OutTempArray` (`self.DefenceTA2Array`))))
  (return (`BlueprintMapLibrary.Map_Find` (`self.SpawnClassMap`) (`local.CharacterType`)) (`local.OutTempArray`)))

(fn `GetPoolCountOfType`
  (params (CharType :type "ECharacterType Enum" :default "ECT_OffenceD"))
  (returns (typeCount :type Integer64))
  (locals (count :type Integer64))
  (bind (_outclass _outarray) (`self.Get Array Class from Enum` CharType))
  (for _array_element _outarray
    (bind _returnvalue (`XR_Character.GetPool` _array_element))
    (if _returnvalue
      (set `local.count` (+ (`local.count`) 1))))
  (return (`local.count`)))

(fn `PoolSpawnActor`
  (params (CharType :type "ECharacterType Enum" :default "ECT_OffenceD"))
  (returns (outCharacter :type "XR_Character Object Reference"))
  (locals (count :type Integer64))
  (bind (_outclass _outarray) (`self.Get Array Class from Enum` CharType))
  (for _array_element _outarray
    (bind _returnvalue (`XR_Character.GetPool` _array_element))
    (if _returnvalue
      (`XR_Character.SetPool` _array_element false)
      (return _array_element)))
  (return null))

(fn `UserConstructionScript`)