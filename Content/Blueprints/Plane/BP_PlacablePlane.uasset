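; BP_PlacablePlane is a placement plane typed as Offence, Defence or Neutral that appears only while an object of the matching type is being grabbed.
; On BeginPlay, its PlaneType selects the mesh and the trace channel it blocks, then the mesh is hidden.
; It registers with BP_GamePlayMode's object grab event, which toggles visibility as a matching grab starts and ends.
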(event `self.ReceiveBeginPlay`
  (`|ExecutionSequence`
    (:`then_0`
      (switch `EObjectType` (`self.PlaneType`)
        (:`EOT_Offence`
          (`StaticMeshComponent.SetStaticMesh` (`self.StaticMesh`) (`self.OffenceMesh`))
          (`PrimitiveComponent.SetCollisionResponseToChannel` (`self.StaticMesh`) "ECC_GameTraceChannel4" "ECR_Block"))
        (:`EOT_Deffence`
          (`StaticMeshComponent.SetStaticMesh` (`self.StaticMesh`) (`self.DeffenceMesh`))
          (`PrimitiveComponent.SetCollisionResponseToChannel` (`self.StaticMesh`) "ECC_GameTraceChannel5" "ECR_Block"))
        (:`EOT_Neutral`
          (`StaticMeshComponent.SetStaticMesh` (`self.StaticMesh`) (`self.NeutralMesh`))
          (`PrimitiveComponent.SetCollisionResponseToChannel` (`self.StaticMesh`) "ECC_GameTraceChannel2" "ECR_Block")))
      (`SceneComponent.SetVisibility` (`self.StaticMesh`) false false)
      (bind _asbp_game_play_mode (cast `/Game/Blueprints/GameMode/BP_GamePlayMode` (`GameplayStatics.GetGameMode`)))
      (set `self.As BP Game Play Mode` _asbp_game_play_mode))
    (:`then_1`
      (bind _as_bp_game_play_mode (`self.As BP Game Play Mode`)
        (:`then`
          (add `/Game/Blueprints/GameMode/BP_GamePlayMode.ObjectGrabEvent` _as_bp_game_play_mode (delegate `ObjectGrabEvent_이벤트`)))
        (:`else`)))))

(event `ObjectGrabEvent_이벤트`
  (params (GrabObjectType :type "EObjectType Enum" :default "EOT_Offence") (isGrabStart :type Boolean))
  (if (`|EnumEquality` GrabObjectType (`self.PlaneType`))
    (`SceneComponent.SetVisibility` (`self.StaticMesh`) isGrabStart false)))

(fn `UserConstructionScript`)