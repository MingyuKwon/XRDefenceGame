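; BP_MapLocationIndicator is an actor that marks the local board's position in an XR defence game, with a text widget label.
; On BeginPlay it moves itself to the board location and rotation stored in XRDefenceGameInstance.
; It writes "DEFENCE" and then "Enemy" to the same DefenceText widget, so "Enemy" remains.
; The construction script also sets that label to "Enemy".
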(event `self.ReceiveBeginPlay`
  (`|ExecutionSequence`
    (:`then_0`
      (bind _aswbp_text (cast `/Game/Blueprints/UI/Hand/WBP_TEXT` (`WidgetComponent.GetWidget` (`self.DefenceText`))))
      (`/Game/Blueprints/UI/Hand/WBP_TEXT.SetText` _aswbp_text "DEFENCE")
      (bind _aswbp_text_2 (cast `/Game/Blueprints/UI/Hand/WBP_TEXT` (`WidgetComponent.GetWidget` (`self.DefenceText`))))
      (`/Game/Blueprints/UI/Hand/WBP_TEXT.SetText` _aswbp_text_2 "Enemy"))
    (:`then_1`
      (bind _asxrdefence_game_instance (cast `XRDefenceGameInstance` (`GameplayStatics.GetGameInstance`)))
      (`self.K2_SetActorLocationAndRotation` (`XRDefenceGameInstance.LocalBoardLocation` _asxrdefence_game_instance) (`XRDefenceGameInstance.LocalBoardRotation` _asxrdefence_game_instance)))))

(fn `UserConstructionScript`
  (bind _aswbp_text (cast `/Game/Blueprints/UI/Hand/WBP_TEXT` (`WidgetComponent.GetWidget` (`self.DefenceText`))))
  (`/Game/Blueprints/UI/Hand/WBP_TEXT.SetText` _aswbp_text "Enemy"))