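; BP_MapSpawner is a map placement actor with a "DEFENCE" label that sets where the XR defence game will be played.
; It binds to MapLocationSetGameMode events, rotating its root in yaw and moving it as they fire.
; On the spawn event, if it has authority and is enabled, it saves the FloorMesh transform to the game instance, calls MoveToLobby on the game mode and destroys itself.
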(event `self.ReceiveBeginPlay`
  (`|ExecutionSequence`
    (:`then_0`
      (bind _asmap_location_set_game_mode (cast `MapLocationSetGameMode` (`GameplayStatics.GetGameMode`)))
      (set `self.As Map Location Set Game Mode` _asmap_location_set_game_mode)
      (bind _aswbp_text (cast `/Game/Blueprints/UI/Hand/WBP_TEXT` (`WidgetComponent.GetWidget` (`self.DefenceText`))))
      (`/Game/Blueprints/UI/Hand/WBP_TEXT.SetText` _aswbp_text "DEFENCE"))
    (:`then_1`
      (bind _as_map_location_set_game_mode (`self.As Map Location Set Game Mode`)
        (:`then`
          (add `MapLocationSetGameMode.OnMapRotateEvent` _as_map_location_set_game_mode (delegate `OnMapRotateEvent_이벤트_0`))
          (bind _as_map_location_set_game_mode_2 (`self.As Map Location Set Game Mode`)
            (:`then`
              (add `MapLocationSetGameMode.OnMapLocationEvent` _as_map_location_set_game_mode_2 (delegate `OnMapLocationEvent_이벤트_0`))
              (bind _as_map_location_set_game_mode_3 (`self.As Map Location Set Game Mode`)
                (:`then`
                  (add `MapLocationSetGameMode.OnMapSpawnEvent` _as_map_location_set_game_mode_3 (delegate `OnMapSpawnEvent_이벤트_0`)))
                (:`else`)))
            (:`else`)))
        (:`else`)))))

(event `OnMapRotateEvent_이벤트_0`
  (params (RotateAmount :type "Float (single-precision)"))
  (`SceneComponent.K2_AddWorldRotation` (`self.DefaultSceneRoot`) (`KismetMathLibrary.MakeRotator` 0.0 0.0 RotateAmount) false false))

(event `OnMapLocationEvent_이벤트_0`
  (params (SpawnLocation :type "Vector Structure"))
  (`SceneComponent.K2_SetWorldLocation` (`self.DefaultSceneRoot`) SpawnLocation false false))

(event `OnMapSpawnEvent_이벤트_0`
  (`self.SpawnMap`))

(event `SpawnMap`
  (bind (_returnvalue_location _returnvalue_rotation) (`KismetMathLibrary.BreakTransform` (`SceneComponent.K2_GetComponentToWorld` (`self.FloorMesh`))))
  (if (`self.HasAuthority`)
    (if (`self.isEnable`)
      (bind _asxrdefence_game_instance (cast `XRDefenceGameInstance` (`GameplayStatics.GetGameInstance`)))
      (set `XRDefenceGameInstance.PlayerGamePlayLocation` _returnvalue_location _asxrdefence_game_instance)
      (set `XRDefenceGameInstance.PlayerGamePlayRotation` _returnvalue_rotation _asxrdefence_game_instance)
      (bind _as_map_location_set_game_mode (`self.As Map Location Set Game Mode`)
        (:`then`
          (`MapLocationSetGameMode.MoveToLobby` _as_map_location_set_game_mode)
          (`self.K2_DestroyActor`))
        (:`else`)))))

(fn `UserConstructionScript`
  (bind _aswbp_text (cast `/Game/Blueprints/UI/Hand/WBP_TEXT` (`WidgetComponent.GetWidget` (`self.DefenceText`))))
  (`/Game/Blueprints/UI/Hand/WBP_TEXT.SetText` _aswbp_text "DEFENCE"))