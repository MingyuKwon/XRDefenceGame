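; BPC_SpawnFloor is a scene component that serves as a spawn point for XR characters.
; SpawnXRCharacter asks the supplied GameMode for an actor of SpawnCharacterType through PoolSpawnActor, so spawning goes through pooling.
; A valid actor is moved slightly above the component's world location, takes its rotation, keeps its own scale and is returned.
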(fn `SpawnXRCharacter`
  (params (GameMode :type "/Game/Blueprints/GameMode/BP_XRGamePlayMode Object Reference"))
  (returns (SpawnActor :type "XR_Character Object Reference"))
  (bind _returnvalue (`XRGamePlayMode.PoolSpawnActor` GameMode (`self.SpawnCharacterType`)))
  (if (`KismetSystemLibrary.IsValid` _returnvalue)
    (`Actor.K2_SetActorTransform` _returnvalue (`KismetMathLibrary.MakeTransform` (+ (`self.K2_GetComponentLocation`) (0.0 0.0 5.0)) (`self.K2_GetComponentRotation`) (`Actor.GetActorScale3D` _returnvalue)) false false)
    (return _returnvalue)
    (else
      (return null))))