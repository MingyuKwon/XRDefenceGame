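; Character palette that stocks six spawn floors with offence or defence characters one second after BeginPlay, based on its ObjectType.
; Offence floors choose a type from their space type (gold, puppet, turret or random offence) and look up its class in a map.
; Each of these characters stores its floor index and binds a set-on-board callback that respawns on that floor.
; The defence path directly spawns BP_XRCharDefence without that callback.
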(event `self.ReceiveBeginPlay`
  (`|ExecutionSequence`
    (:`then_0`
      (`KismetArrayLibrary.Array_Add` (`self.SpawnFloorArray`) (`self.BPC_SpawnFloor1`))
      (`KismetArrayLibrary.Array_Add` (`self.SpawnFloorArray`) (`self.BPC_SpawnFloor2`))
      (`KismetArrayLibrary.Array_Add` (`self.SpawnFloorArray`) (`self.BPC_SpawnFloor3`))
      (`KismetArrayLibrary.Array_Add` (`self.SpawnFloorArray`) (`self.BPC_SpawnFloor4`))
      (`KismetArrayLibrary.Array_Add` (`self.SpawnFloorArray`) (`self.BPC_SpawnFloor5`))
      (`KismetArrayLibrary.Array_Add` (`self.SpawnFloorArray`) (`self.BPC_SpawnFloor6`)))
    (:`then_1`
      (`KismetSystemLibrary.K2_SetTimerDelegate` (delegate `커스텀이벤트`) 1.0))))

(event `커스텀이벤트`
  (switch `EObjectType` (`self.ObjectType`)
    (:`EOT_Offence`
      (`self.SpawnALLOffenceChar`))
    (:`EOT_Deffence`
      (`self.SpawnALLDefenceChar`))))

(event `AssignBoardCallBackToActor`
  (params (SpawnActor :type "XR_Character Object Reference") (Index :type Integer))
  (`XR_Character.SetSpawnPlaceIndex` SpawnActor Index)
  (add `XR_Character.OnSetBoardEvent` SpawnActor (delegate `OnSetBoardEvent_이벤트`)))

(event `OnSetBoardEvent_이벤트`
  (params (objectType :type "EObjectType Enum" :default "EOT_Offence") (characterType :type "ECharacterType Enum" :default "ECT_OffenceD") (SpawnPlaceIndex :type Integer))
  (`self.SpawnSpecificFloor` (`|GetArrayItem` (`self.SpawnFloorArray`) SpawnPlaceIndex)))

(fn `Get Next Spawn Character Type`
  (params (SpawnFloor :type "/Game/Blueprints/Palette/BPC_SpawnFloor Object Reference"))
  (returns (OutType :type "ECharacterType Enum"))
  (locals (outCharacterType :type "ECharacterType Enum" :default "ECT_OffenceD"))
  (switch `/Game/Blueprints/Palette/EPalleteSlotType` (`/Game/Blueprints/Palette/BPC_SpawnFloor.PalletSpaceType` SpawnFloor)
    (:`NewEnumerator0`
      (set `local.outCharacterType` "ECT_Gold"))
    (:`NewEnumerator1`
      (set `local.outCharacterType` "ECT_DefenceP"))
    (:`NewEnumerator2`
      (set `local.outCharacterType` "ECT_DefenceT"))
    (:`NewEnumerator3`
      (switch `EObjectType` (`self.ObjectType`)
        (:`EOT_Offence`
          (set `local.outCharacterType` (`KismetArrayLibrary.Array_Random` (`self.OffenceCharTypes`)))))))
  (return (`local.outCharacterType`)))

(fn `SpawnALLDefenceChar`
  (`|ExecutionSequence`
    (:`then_0`
      (set `/Game/Blueprints/Palette/BPC_SpawnFloor.SpawnCharacterClass` "/Game/Blueprints/Characters/Defence/BP_XRCharDefence.BP_XRCharDefence_C" (`self.BPC_SpawnFloor1`))
      (`/Game/Blueprints/Palette/BPC_SpawnFloor.SpawnXRCharacter` (`self.BPC_SpawnFloor1`)))
    (:`then_1`
      (set `/Game/Blueprints/Palette/BPC_SpawnFloor.SpawnCharacterClass` "/Game/Blueprints/Characters/Defence/BP_XRCharDefence.BP_XRCharDefence_C" (`self.BPC_SpawnFloor2`))
      (`/Game/Blueprints/Palette/BPC_SpawnFloor.SpawnXRCharacter` (`self.BPC_SpawnFloor2`)))
    (:`then_2`
      (set `/Game/Blueprints/Palette/BPC_SpawnFloor.SpawnCharacterClass` "/Game/Blueprints/Characters/Defence/BP_XRCharDefence.BP_XRCharDefence_C" (`self.BPC_SpawnFloor3`))
      (`/Game/Blueprints/Palette/BPC_SpawnFloor.SpawnXRCharacter` (`self.BPC_SpawnFloor3`)))
    (:`then_3`
      (set `/Game/Blueprints/Palette/BPC_SpawnFloor.SpawnCharacterClass` "/Game/Blueprints/Characters/Defence/BP_XRCharDefence.BP_XRCharDefence_C" (`self.BPC_SpawnFloor4`))
      (`/Game/Blueprints/Palette/BPC_SpawnFloor.SpawnXRCharacter` (`self.BPC_SpawnFloor4`)))
    (:`then_4`
      (set `/Game/Blueprints/Palette/BPC_SpawnFloor.SpawnCharacterClass` "/Game/Blueprints/Characters/Defence/BP_XRCharDefence.BP_XRCharDefence_C" (`self.BPC_SpawnFloor5`))
      (`/Game/Blueprints/Palette/BPC_SpawnFloor.SpawnXRCharacter` (`self.BPC_SpawnFloor5`)))
    (:`then_5`
      (set `/Game/Blueprints/Palette/BPC_SpawnFloor.SpawnCharacterClass` "/Game/Blueprints/Characters/Defence/BP_XRCharDefence.BP_XRCharDefence_C" (`self.BPC_SpawnFloor6`))
      (`/Game/Blueprints/Palette/BPC_SpawnFloor.SpawnXRCharacter` (`self.BPC_SpawnFloor6`)))))

(fn `SpawnALLOffenceChar`
  (`|ExecutionSequence`
    (:`then_0`
      (`self.SpawnSpecificFloor` (`self.BPC_SpawnFloor1`)))
    (:`then_1`
      (`self.SpawnSpecificFloor` (`self.BPC_SpawnFloor2`)))
    (:`then_2`
      (`self.SpawnSpecificFloor` (`self.BPC_SpawnFloor3`)))
    (:`then_3`
      (`self.SpawnSpecificFloor` (`self.BPC_SpawnFloor4`)))
    (:`then_4`
      (`self.SpawnSpecificFloor` (`self.BPC_SpawnFloor5`)))
    (:`then_5`
      (`self.SpawnSpecificFloor` (`self.BPC_SpawnFloor6`)))))

(fn `SpawnOnPlace`
  (params (SpawnFloor :type "/Game/Blueprints/Palette/BPC_SpawnFloor Object Reference") (CharacterType :type "ECharacterType Enum" :default "ECT_OffenceD"))
  (set `/Game/Blueprints/Palette/BPC_SpawnFloor.SpawnCharacterClass` (`BlueprintMapLibrary.Map_Find` (`self.SpawnClassMap`) CharacterType) SpawnFloor)
  (bind _spawnactor (`/Game/Blueprints/Palette/BPC_SpawnFloor.SpawnXRCharacter` SpawnFloor))
  (`self.AssignBoardCallBackToActor` _spawnactor (`KismetArrayLibrary.Array_Find` (`self.SpawnFloorArray`) SpawnFloor)))

(fn `SpawnSpecificFloor`
  (params (SpawnFloor :type "/Game/Blueprints/Palette/BPC_SpawnFloor Object Reference"))
  (bind _outtype (`self.Get Next Spawn Character Type` SpawnFloor))
  (`self.SpawnOnPlace` SpawnFloor _outtype))

(fn `UserConstructionScript`)