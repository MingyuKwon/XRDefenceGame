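; Surrender button actor that triggers a pawn's surrender after five one-second ticks of overlap.
; Box overlaps count BP_GamePlayPawn actors whose controller object type matches ObjectType, starting a looping timer on the first.
; Each tick increments Countdown, updates the WBP_Surrender widget's progress and calls TriggerSurrender at five.
; When the last overlap ends, the timer clears and displayed progress resets, but Countdown keeps its value.
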(event `OnComponentEndOverlap_이벤트`
  (params (OverlappedComponent :type "PrimitiveComponent Object Reference") (OtherActor :type "Actor Object Reference") (OtherComp :type "PrimitiveComponent Object Reference") (OtherBodyIndex :type Integer))
  (bind _asbp_game_play_pawn (cast `/Game/Blueprints/Player/Pawns/BP_GamePlayPawn` OtherActor))
  (bind _newparam (`/Game/Blueprints/Player/Pawns/BP_GamePlayPawn.GetControllerObjectType` _asbp_game_play_pawn))
  (if (`|EnumEquality` _newparam (`self.ObjectType`))
    (bind _output_get (set `self.refCount` (+ (`self.refCount`) -1)))
    (if (== _output_get 0)
      (`self.OverlapEnd`)
      (set `self.As BP Game Play Pawn` null))))

(event `self.ReceiveBeginPlay`
  (bind _box (`self.Box`))
  (bind _aswbp_surrender (cast `/Game/Blueprints/UI/WBP_Surrender` (`WidgetComponent.GetWidget` (`self.Widget`))))
  (set `self.As WBP Surrender` _aswbp_surrender)
  (add `PrimitiveComponent.OnComponentBeginOverlap` _box (delegate `OnComponentBeginOverlap_이벤트`))
  (add `PrimitiveComponent.OnComponentEndOverlap` _box (delegate `OnComponentEndOverlap_이벤트`)))

(event `OnComponentBeginOverlap_이벤트`
  (params (OverlappedComponent :type "PrimitiveComponent Object Reference") (OtherActor :type "Actor Object Reference") (OtherComp :type "PrimitiveComponent Object Reference") (OtherBodyIndex :type Integer) (bFromSweep :type Boolean) (SweepResult :type "HitResult Structure (by ref)"))
  (bind _asbp_game_play_pawn (cast `/Game/Blueprints/Player/Pawns/BP_GamePlayPawn` OtherActor))
  (bind _newparam (`/Game/Blueprints/Player/Pawns/BP_GamePlayPawn.GetControllerObjectType` _asbp_game_play_pawn))
  (if (`|EnumEquality` _newparam (`self.ObjectType`))
    (bind _output_get (set `self.refCount` (+ (`self.refCount`) 1)))
    (if (== _output_get 1)
      (set `self.As BP Game Play Pawn` _asbp_game_play_pawn)
      (`self.OverlapStart`))))

(event `OverlapStart`
  (bind _returnvalue (`KismetSystemLibrary.K2_SetTimerDelegate` (delegate `커스텀이벤트`) 1.0 true))
  (set `self.SurrenderHandler` _returnvalue))

(event `커스텀이벤트`
  (bind _output_get (set `self.countdown` (+ (`self.countdown`) 1)))
  (bind _as_wbp_surrender (`self.As WBP Surrender`)
    (:`then`
      (`/Game/Blueprints/UI/WBP_Surrender.ProgressUpdate` _as_wbp_surrender (`KismetMathLibrary.Conv_IntToDouble` _output_get))
      (if (== _output_get 5)
        (set `self.SurrenderHandler` (struct))
        (bind _as_bp_game_play_pawn (`self.As BP Game Play Pawn`)
          (:`then`
            (`PlayerPawn.TriggerSurrender` _as_bp_game_play_pawn))
          (:`else`))))
    (:`else`)))

(event `OverlapEnd`
  (bind _surrenderhandler (`self.SurrenderHandler`))
  (if (`KismetSystemLibrary.K2_IsValidTimerHandle` _surrenderhandler)
    (`KismetSystemLibrary.K2_ClearAndInvalidateTimerHandle` _surrenderhandler)
    (bind _as_wbp_surrender (`self.As WBP Surrender`)
      (:`then`
        (`/Game/Blueprints/UI/WBP_Surrender.ProgressUpdate` _as_wbp_surrender 0.0))
      (:`else`))))

(fn `UserConstructionScript`)