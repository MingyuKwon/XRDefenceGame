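; Hand-tracked XR player pawn for a defence game, with shoot, stun and speed-change abilities plus wrist-watch UI.
; Tick sends recognized poses and right-hand gestures to BP_PlayerController and tints hands by pose.
; Action events swap pose confidence floors and toggle line-traced Niagara aiming for held gestures.
; Follow-up gestures fire or change speed by team role, while hitting the floor triggers stun, all gated by the controller's shared cooldown.
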(event `Key|Q`
  (params (Key :type "Key Structure"))
  (:`Pressed`
    (`KismetSystemLibrary.QuitGame` null "Quit")))

(event `self.PoseRightAction`
  (params (currentPose :type "Pose Enum" :default "Grab"))
  (`self.RightPoseAction` currentPose))

(event `self.SetUBlueHealth`
  (params (HealthAmount :type "Float (single-precision)"))
  ;[1 1 1] UI CHange
  (bind _as_wbp_hand_watch_ui (`self.As WBP Hand Watch UI`)
    (:`then`
      (`GamePlayHandUI.SetBlueHeartText` _as_wbp_hand_watch_ui HealthAmount))
    (:`else`)))

(event `InputAction|LogLeftHand`
  (params (Key :type "Key Structure"))
  ;[1 1 1] HandPoseLog
  (:`Released`
    (`HandPoseRecognizer.LogEncodedHandPose` (`self.LeftHandPoseRecognizer`))))

(event `RightPoseThresholdChange`
  (params (isDefault :type Boolean))
  ;[1 1 1] HandPoseRecognize Threshold Change
  (if isDefault
    (set `HandPoseRecognizer.DefaultConfidenceFloor` (`self.PoseDefaultThreshold`) (`self.RightHandPose`))
    (else
      (set `HandPoseRecognizer.DefaultConfidenceFloor` (`self.PoseActivatingThreshold`) (`self.RightHandPose`)))))

(event `self.PoseLeftAction`
  (params (currentPose :type "Pose Enum" :default "Grab"))
  (`self.LeftPoseAction` currentPose))

(event `self.SetRightHandPosition`
  (set `self.RightHandPosition` (`SceneComponent.K2_GetComponentLocation` (`self.RightCollision`))))

(event `self.SetUIGoldAmount`
  (params (GoldAmount :type "Float (single-precision)") (MaxGoldAmount :type "Float (single-precision)"))
  ;[1 1 1] UI CHange
  (bind _as_wbp_hand_watch_ui (`self.As WBP Hand Watch UI`)
    (:`then`
      (`GamePlayHandUI.SetGoldText` _as_wbp_hand_watch_ui GoldAmount MaxGoldAmount))
    (:`else`)))

(event `InputAction|LogRightHand`
  (params (Key :type "Key Structure"))
  ;[1 1 1] HandPoseLog
  (:`Released`
    (`HandPoseRecognizer.LogEncodedHandPose` (`self.RightHandPoseRecognizer`))))

(event `LeftPoseThresholdChange`
  (params (isDefault :type Boolean))
  ;[1 1 1] HandPoseRecognize Threshold Change
  (if isDefault
    (set `HandPoseRecognizer.DefaultConfidenceFloor` (`self.PoseDefaultThreshold`) (`self.LeftHandPose`))
    (else
      (set `HandPoseRecognizer.DefaultConfidenceFloor` (`self.PoseActivatingThreshold`) (`self.LeftHandPose`)))))

(event `self.GestureRightAction`
  (params (currentGesture :type "EGesture Enum" :default "Rock_Scissors"))
  (`self.RightGestureAction` currentGesture))

(event `self.SetUIHealth`
  (params (HealthAmount :type "Float (single-precision)"))
  ;[1 1 1] UI CHange
  (bind _as_wbp_hand_watch_ui (`self.As WBP Hand Watch UI`)
    (:`then`
      (`GamePlayHandUI.SetHealthText` _as_wbp_hand_watch_ui HealthAmount))
    (:`else`)))

(event `self.SetLeftHandPosition`
  (set `self.LeftHandPosition` (`SceneComponent.K2_GetComponentLocation` (`self.LeftCollision`))))

(event `self.ReleaseGestureRight`
  (params (currentGesture :type "EGesture Enum" :default "Rock_Scissors"))
  (`self.RightGestureReleaseFunc` currentGesture))

(event `self.SetUIOrnageHealth`
  (params (HealthAmount :type "Float (single-precision)"))
  ;[1 1 1] UI CHange
  (bind _as_wbp_hand_watch_ui (`self.As WBP Hand Watch UI`)
    (:`then`
      (`GamePlayHandUI.SetOrangeHeartText` _as_wbp_hand_watch_ui HealthAmount))
    (:`else`)))

(event `self.SetUIPurpleHealth`
  (params (HealthAmount :type "Float (single-precision)"))
  ;[1 1 1] UI CHange
  (bind _as_wbp_hand_watch_ui (`self.As WBP Hand Watch UI`)
    (:`then`
      (`GamePlayHandUI.SetPurpleHeartText` _as_wbp_hand_watch_ui HealthAmount))
    (:`else`)))

(event `self.SetUITime`
  (params (TimeSecond :type "Float (single-precision)"))
  ;[1 1 1] UI CHange
  (bind _as_wbp_hand_watch_ui (`self.As WBP Hand Watch UI`)
    (:`then`
      (`GamePlayHandUI.SetTimeText` _as_wbp_hand_watch_ui TimeSecond))
    (:`else`)))

(event `self.ReceiveBeginPlay`
  (bind _returnvalue (`self.GetController`))
  (bind _leftcollision (`self.LeftCollision`))
  (bind _rightcollision (`self.RightCollision`))
  (if (`KismetSystemLibrary.IsValid` _returnvalue)
    (if (`Controller.IsLocalPlayerController` _returnvalue)
      (`parent.ReceiveBeginPlay`)
      (`|ExecutionSequence`
        (:`then_0`
          (bind _asbp_player_controller (cast `/Game/Blueprints/Player/Controller/BP_PlayerController` (`self.GetController`)))
          (set `self.As BP Player Controller` _asbp_player_controller)
          (bind _asxrdefence_game_instance (cast `XRDefenceGameInstance` (`GameplayStatics.GetGameInstance`)))
          (set `self.As XRDefence Game Instance` _asxrdefence_game_instance)
          (bind _asxrgame_play_mode (cast `XRGamePlayMode` (`GameplayStatics.GetGameMode`)))
          (set `self.As XRGame Play Mode` _asxrgame_play_mode))
        (:`then_1`
          (`self.RightPoseThresholdChange` true)
          (`self.LeftPoseThresholdChange` true))
        (:`then_2`
          (add `PrimitiveComponent.OnComponentBeginOverlap` _rightcollision (delegate `OnComponentBeginOverlap_이벤트`))
          (add `PrimitiveComponent.OnComponentEndOverlap` _rightcollision (delegate `OnComponentEndOverlap_이벤트`)))
        (:`then_3`
          (add `PrimitiveComponent.OnComponentBeginOverlap` _leftcollision (delegate `OnComponentBeginOverlap_이벤트_0`))
          (add `PrimitiveComponent.OnComponentEndOverlap` _leftcollision (delegate `OnComponentEndOverlap_이벤트_0`)))
        (:`then_4`
          (bind _aswbp_left_hand_watch_ui (cast `/Game/Blueprints/UI/Hand/WBP_LeftHandWatchUI` (`WidgetComponent.GetWidget` (`self.LeftWatchUI`))))
          (set `self.As WBP Hand Watch UI` _aswbp_left_hand_watch_ui)
          (bind _aswbp_right_hand_watch_ui (cast `/Game/Blueprints/UI/Hand/WBP_RightHandWatchUI` (`WidgetComponent.GetWidget` (`self.RightWatchUI`))))
          (set `self.As WBP Right Hand Watch UI` _aswbp_right_hand_watch_ui))
        (:`then_5`
          (add `PrimitiveComponent.OnComponentBeginOverlap` (`self.HitCollisionRight`) (delegate `OnComponentBeginOverlap_이벤트_1`)))
        (:`then_6`
          (`SceneComponent.SetVisibility` (`self.ShootAreaShowNiagara`) false false)
          (`SceneComponent.SetVisibility` (`self.StunAreaShowNiagara`) false false)
          (`SceneComponent.SetVisibility` (`self.SpeedBuffAreaShowNiagara`) false false)))
      (else
        (`SceneComponent.SetVisibility` (`self.DefaultSceneRoot`) false true :!label _label)))
    (else
      (goto _label))))

(event `self.SetUIGestureCoolTime`
  (params (percent :type "Float (single-precision)"))
  ;[1 1 1] UI CHange
  (bind _as_wbp_right_hand_watch_ui (`self.As WBP Right Hand Watch UI`)
    (:`then`
      (`GestureDisplayWatch.SetCoolTimeProgressBar` _as_wbp_right_hand_watch_ui percent))
    (:`else`)))

(event `OnComponentEndOverlap_이벤트`
  (params (OverlappedComponent :type "PrimitiveComponent Object Reference") (OtherActor :type "Actor Object Reference") (OtherComp :type "PrimitiveComponent Object Reference") (OtherBodyIndex :type Integer))
  (bind _ashand_interact_interface (cast `HandInteractInterface` OtherActor))
  (bind _as_bp_player_controller (`self.As BP Player Controller`)
    (:`then`
      (`Player_Controller.HandInteractRightOverlapEnd` _as_bp_player_controller _ashand_interact_interface))
    (:`else`)))

(event `OnComponentBeginOverlap_이벤트`
  (params (OverlappedComponent :type "PrimitiveComponent Object Reference") (OtherActor :type "Actor Object Reference") (OtherComp :type "PrimitiveComponent Object Reference") (OtherBodyIndex :type Integer) (bFromSweep :type Boolean) (SweepResult :type "HitResult Structure (by ref)"))
  (bind _ashand_interact_interface (cast `HandInteractInterface` OtherActor))
  (bind _as_bp_player_controller (`self.As BP Player Controller`)
    (:`then`
      (`Player_Controller.HandInteractRightOverlapStart` _as_bp_player_controller _ashand_interact_interface))
    (:`else`)))

(event `self.ReceiveTick`
  (params (DeltaSeconds :type "Float (single-precision)"))
  (if (`SceneComponent.IsVisible` (`self.DefaultSceneRoot`))
    (`|ExecutionSequence`
      (:`then_0`
        (bind (_index _name _duration _error _confidence _returnvalue) (`HandPoseRecognizer.GetRecognizedHandPose` (`self.RightHandPose`)))
        (`self.RightPoseInputCheck` _name _returnvalue)
        (bind (_index_2 _name_2 _gesturedirection _gestureouterduration _gestureinnerduration _returnvalue_2) (`HandGestureRecognizer.GetRecognizedHandGesture` (`self.RightHandGesture`) "Reset"))
        (`self.Right Gesture` _name_2 _returnvalue_2)
        (bind (_index_3 _name_3 _duration_2 _error_2 _confidence_2 _returnvalue_3) (`HandPoseRecognizer.GetRecognizedHandPose` (`self.LeftHandPose`)))
        (`self.LeftPoseInputCheck` _name_3 _returnvalue_3))
      (:`then_1`
        (bind _as_bp_player_controller (`self.As BP Player Controller`)
          (:`then`
            (bind _returnvalue_4 (`Player_Controller.IsGestureWorkable` _as_bp_player_controller))
            (if _returnvalue_4
              (`self.CheckShootLine`)
              (`self.CheckStunLine`)
              (`self.CheckSpeedBuffLine`)))
          (:`else`))))))

(event `OnComponentBeginOverlap_이벤트_0`
  (params (OverlappedComponent :type "PrimitiveComponent Object Reference") (OtherActor :type "Actor Object Reference") (OtherComp :type "PrimitiveComponent Object Reference") (OtherBodyIndex :type Integer) (bFromSweep :type Boolean) (SweepResult :type "HitResult Structure (by ref)"))
  (bind _ashand_interact_interface (cast `HandInteractInterface` OtherActor))
  (`Player_Controller.HandInteractLeftOverlapStart` (`self.As BP Player Controller`) _ashand_interact_interface))

(event `OnComponentEndOverlap_이벤트_0`
  (params (OverlappedComponent :type "PrimitiveComponent Object Reference") (OtherActor :type "Actor Object Reference") (OtherComp :type "PrimitiveComponent Object Reference") (OtherBodyIndex :type Integer))
  (bind _ashand_interact_interface (cast `HandInteractInterface` OtherActor))
  (`Player_Controller.HandInteractLeftOverlapEnd` (`self.As BP Player Controller`) _ashand_interact_interface))

(event `OnComponentBeginOverlap_이벤트_1`
  (params (OverlappedComponent :type "PrimitiveComponent Object Reference") (OtherActor :type "Actor Object Reference") (OtherComp :type "PrimitiveComponent Object Reference") (OtherBodyIndex :type Integer) (bFromSweep :type Boolean) (SweepResult :type "HitResult Structure (by ref)"))
  (cast `/Game/Blueprints/GameMapLevel/BP_BaseFloor` OtherActor)
  (`self.StunArea`))

(fn `Change Hand Color`
  (params (`Material Hand` :type "OculusXRHandComponent Object Reference") (Gesture :type "Pose Enum" :default "Grab"))
  (locals (Material :type "MaterialInterface Object Reference"))
  (switch `Pose` Gesture
    (:`Grab`
      (set `local.Material` (`self.Grab Material`)))
    (:`Rock`
      (set `local.Material` (`self.Rock Material`)))
    (:`scissors`
      (set `local.Material` (`self.Scissor Materail`)))
    (:`Paper`
      (set `local.Material` (`self.Paper Material`)))
    (:`Thumb`
      (set `local.Material` (`self.Thumb Material`)))
    (:`None`
      (set `local.Material` (`self.NULLMaterial`))))
  (`PrimitiveComponent.SetMaterial` (`local.Material Hand`) 0 (`local.Material`)))

(fn `CheckShootLine`
  (bind _returnvalue (`SceneComponent.K2_GetComponentLocation` (`self.ShootAreaShowNiagara`)))
  (bind _returnvalue_2 (+ _returnvalue (* (`SceneComponent.GetForwardVector` (`self.SpeedBuffSphere`)) (-200.0 -200.0 -200.0))))
  (if (`self.NowScissorsGesture`)
    (set `self.FireStartLocation` _returnvalue)
    (`FXSystemComponent.SetVectorParameter` (`self.ShootAreaShowNiagara`) "BeamEnd" _returnvalue_2)
    (bind (_outhit _returnvalue_3) (`KismetSystemLibrary.LineTraceSingle` _returnvalue _returnvalue_2 "TraceTypeQuery4"))
    (if _returnvalue_3
      (set `self.FireEndLocation` (`.ImpactPoint` (`GameplayStatics.BreakHitResult` _outhit)))
      (`SceneComponent.SetVisibility` (`self.ShootAreaShowNiagara`) true false)
      (`FXSystemComponent.SetVectorParameter` (`self.ShootAreaShowNiagara`) "BeamEnd" (`self.FireEndLocation`))
      (bind _returnvalue_4 (`NiagaraFunctionLibrary.SpawnSystemAtLocation` "/Game/Niagara/NS_PlayerSpeedBuffRing.NS_PlayerSpeedBuffRing" (`self.FireEndLocation`)))
      (`FXSystemComponent.SetFloatParameter` _returnvalue_4 "Radius" (`self.AttackRange`))
      (else
        (`SceneComponent.SetVisibility` (`self.ShootAreaShowNiagara`) false false)))))

(fn `CheckSpeedBuffLine`
  (bind _returnvalue (`SceneComponent.K2_GetComponentLocation` (`self.SpeedBuffAreaShowNiagara`)))
  (bind _returnvalue_2 (+ _returnvalue (* (`KismetMathLibrary.Vector_Down`) (200.0 200.0 200.0))))
  (if (`self.NowThumbGesture`)
    (set `self.SpeedStartLocation` _returnvalue)
    (`FXSystemComponent.SetVectorParameter` (`self.SpeedBuffAreaShowNiagara`) "BeamEnd" _returnvalue_2)
    (bind (_outhit _returnvalue_3) (`KismetSystemLibrary.LineTraceSingle` _returnvalue _returnvalue_2 "TraceTypeQuery4"))
    (if _returnvalue_3
      (set `self.SpeedEndLocation` (`.ImpactPoint` (`GameplayStatics.BreakHitResult` _outhit)))
      (`SceneComponent.SetVisibility` (`self.SpeedBuffAreaShowNiagara`) true false)
      (`FXSystemComponent.SetVectorParameter` (`self.SpeedBuffAreaShowNiagara`) "BeamEnd" (`self.SpeedEndLocation`))
      (bind _returnvalue_4 (`NiagaraFunctionLibrary.SpawnSystemAtLocation` "/Game/Niagara/NS_PlayerSpeedBuffRing.NS_PlayerSpeedBuffRing" (`self.SpeedEndLocation`)))
      (`FXSystemComponent.SetFloatParameter` _returnvalue_4 "Radius" (`self.StunRange`))
      (else
        (`SceneComponent.SetVisibility` (`self.SpeedBuffAreaShowNiagara`) false false)))))

(fn `CheckStunLine`
  (bind _returnvalue (`SceneComponent.K2_GetComponentLocation` (`self.StunAreaShowNiagara`)))
  (bind _returnvalue_2 (+ _returnvalue (* (`KismetMathLibrary.Vector_Down`) (200.0 200.0 200.0))))
  (if (`self.CanStun`)
    (set `self.StunStartLocation` _returnvalue)
    (`FXSystemComponent.SetVectorParameter` (`self.StunAreaShowNiagara`) "BeamEnd" _returnvalue_2)
    (bind (_outhit _returnvalue_3) (`KismetSystemLibrary.LineTraceSingle` _returnvalue _returnvalue_2 "TraceTypeQuery4"))
    (if _returnvalue_3
      (set `self.StunEndLocation` (`.ImpactPoint` (`GameplayStatics.BreakHitResult` _outhit)))
      (`SceneComponent.SetVisibility` (`self.StunAreaShowNiagara`) true false)
      (`FXSystemComponent.SetVectorParameter` (`self.StunAreaShowNiagara`) "BeamEnd" (`self.StunEndLocation`))
      (bind _returnvalue_4 (`NiagaraFunctionLibrary.SpawnSystemAtLocation` "/Game/Niagara/NS_PlayerStunRing.NS_PlayerStunRing" (`self.StunEndLocation`)))
      (`FXSystemComponent.SetFloatParameter` _returnvalue_4 "Radius" (`self.StunRange`))
      (else
        (`SceneComponent.SetVisibility` (`self.StunAreaShowNiagara`) false false)))))

(fn `LeftPoseAction`
  (params (InputPose :type "Pose Enum" :default "Grab"))
  (if (`|EnumEquality` InputPose)
    (`self.LeftPoseThresholdChange` true)
    (else
      (`self.LeftPoseThresholdChange` false))))

(fn `LeftPoseInputCheck`
  (params (PoseName :type String) (bPoseRecognized :type Boolean))
  (locals (RecognizePose :type "Pose Enum" :default "scissors"))
  (if bPoseRecognized
    (switch `string` PoseName
      (:`Default`
        (set `local.RecognizePose` "None" :!label _label))
      (:`Grab`
        (set `local.RecognizePose` "Grab"))
      (:`Scissors`
        (set `local.RecognizePose` "scissors"))
      (:`Rock`
        (set `local.RecognizePose` "Rock"))
      (:`Paper`
        (set `local.RecognizePose` "Paper"))
      (:`Thumb`
        (set `local.RecognizePose` "Thumb")))
    (else
      (goto _label)))
  (`self.Change Hand Color` (`self.LeftHand`) (`local.RecognizePose`))
  (bind _as_bp_player_controller (`self.As BP Player Controller`)
    (:`then`
      (`Player_Controller.UpdateCurrentLeftPose` _as_bp_player_controller (`local.RecognizePose`)))
    (:`else`)))

(fn `Right Gesture`
  (params (Selection :type String) (isGestureRecognized :type Boolean))
  (locals (inputGesture :type "EGesture Enum"))
  (if isGestureRecognized
    (switch `string` Selection
      (:`Default`
        (set `local.inputGesture` "None" :!label _label))
      (:`RockScissors`
        (set `local.inputGesture` "Rock_Scissors"))
      (:`RockPaper`
        (set `local.inputGesture` "Rock_Paper"))
      (:`RockThumb`
        (set `local.inputGesture` "Rock_Thumb"))
      (:`ScissorsThumb`
        (set `local.inputGesture` "Scissors_Thumb"))
      (:`ThumbRock`
        (set `local.inputGesture` "Thumb_Rock")))
    (else
      (goto _label)))
  (bind _as_bp_player_controller (`self.As BP Player Controller`)
    (:`then`
      (`Player_Controller.UpdateCurrentRightGesture` _as_bp_player_controller (`local.inputGesture`)))
    (:`else`)))

(fn `RightGestureAction`
  (params (inputGesture :type "EGesture Enum" :default "Rock_Scissors"))
  (switch `EGesture` inputGesture
    (:`Rock_Scissors`
      (set `self.NowScissorsGesture` true)
      (`self.As XRGame Play Mode`
        (:`then`)
        (:`else`)))
    (:`Rock_Paper`
      (set `self.NowPaperGesture` true)
      (`self.As XRGame Play Mode`
        (:`then`
          (set `self.CanStun` true))
        (:`else`)))
    (:`Rock_Thumb`
      (set `self.NowThumbGesture` true))
    (:`Scissors_Thumb`
      (`self.As XRGame Play Mode`
        (:`then`
          (`self.ShootDamage`))
        (:`else`)))
    (:`Thumb_Rock`
      (`self.As XRGame Play Mode`
        (:`then`
          (`self.SpeedBuffArea`))
        (:`else`)))))

(fn `RightGestureReleaseFunc`
  (params (inputGesture :type "EGesture Enum" :default "Rock_Scissors"))
  (switch `EGesture` inputGesture
    (:`Rock_Scissors`
      (set `self.NowScissorsGesture` false)
      (`SceneComponent.SetVisibility` (`self.ShootAreaShowNiagara`) false false))
    (:`Rock_Paper`
      (set `self.NowPaperGesture` false)
      (`SceneComponent.SetVisibility` (`self.StunAreaShowNiagara`) false false)
      (set `self.CanStun` false))
    (:`Rock_Thumb`
      (set `self.NowThumbGesture` false)
      (`SceneComponent.SetVisibility` (`self.SpeedBuffAreaShowNiagara`) false false))))

(fn `RightPoseAction`
  (params (InputPose :type "Pose Enum" :default "Grab"))
  (if (`|EnumEquality` InputPose)
    (`self.RightPoseThresholdChange` true)
    (else
      (`self.RightPoseThresholdChange` false))))

(fn `RightPoseInputCheck`
  (params (PoseName :type String) (bPoseRecognized :type Boolean))
  (locals (RecognizePose :type "Pose Enum" :default "None"))
  (if bPoseRecognized
    (switch `string` PoseName
      (:`Default`
        (set `local.RecognizePose` "None" :!label _label))
      (:`Grab`
        (set `local.RecognizePose` "Grab"))
      (:`Scissors`
        (set `local.RecognizePose` "scissors"))
      (:`Rock`
        (set `local.RecognizePose` "Rock"))
      (:`Paper`
        (set `local.RecognizePose` "Paper"))
      (:`Thumb`
        (set `local.RecognizePose` "Thumb")))
    (else
      (goto _label)))
  (`self.Change Hand Color` (`self.RightHand`) (`local.RecognizePose`))
  (bind _as_bp_player_controller (`self.As BP Player Controller`)
    (:`then`
      (`Player_Controller.UpdateCurrentRightPose` _as_bp_player_controller (`local.RecognizePose`)))
    (:`else`)))

(fn `ShootDamage`
  (bind _as_bp_player_controller (`self.As BP Player Controller`)
    (:`then`
      (bind _returnvalue (`Player_Controller.IsGestureWorkable` _as_bp_player_controller))
      (if _returnvalue
        (if (`Player_Controller.bcanFire` _as_bp_player_controller)
          (bind _returnvalue_2 (`|SpawnActorFromClass` "/Game/Blueprints/Battle/BP_PlayerFire.BP_PlayerFire_C" (`KismetMathLibrary.MakeTransform` (`self.FireStartLocation`) (`KismetMathLibrary.Conv_VectorToRotator` (`KismetMathLibrary.Vector_NormalUnsafe` (- (`self.FireEndLocation`) (`self.FireStartLocation`))))) "Undefined" "MultiplyWithRoot" null null))
          (`Projectile.SetDamage` _returnvalue_2 (`self.AttackDamage`))
          (`Projectile.SetTarget` _returnvalue_2 (`self.FireEndLocation`))
          (`Player_Controller.SetGestureCoolTime` _as_bp_player_controller))))
    (:`else`)))

(fn `SpeedBuffArea`
  (bind _as_bp_player_controller (`self.As BP Player Controller`)
    (:`then`
      (bind _returnvalue (`Player_Controller.IsGestureWorkable` _as_bp_player_controller))
      (if _returnvalue
        (if (`Player_Controller.bcanSpeedBuff` _as_bp_player_controller)
          (`SceneComponent.SetVisibility` (`self.SpeedBuffAreaShowNiagara`) false false)
          (`Player_Controller.SetGestureCoolTime` _as_bp_player_controller)
          (bind _as_bp_player_controller_2 (`self.As BP Player Controller`)
            (:`then`
              (bind _controllerobjecttype (`Player_Controller.controllerObjectType` _as_bp_player_controller_2))
              (switch `EObjectType` _controllerobjecttype
                (:`EOT_Offence`
                  (bind _returnvalue_2 (`NiagaraFunctionLibrary.SpawnSystemAtLocation` "/Game/Niagara/NS_SpeedBuffRangeRingFast.NS_SpeedBuffRangeRingFast" (`self.SpeedEndLocation`)))
                  (`FXSystemComponent.SetFloatParameter` _returnvalue_2 "Radius" (`self.SpeedBuffRange`)))
                (:`EOT_Deffence`
                  (bind _returnvalue_3 (`NiagaraFunctionLibrary.SpawnSystemAtLocation` "/Game/Niagara/NS_SpeedBuffRangeRingSlow.NS_SpeedBuffRangeRingSlow" (`self.SpeedEndLocation`)))
                  (`FXSystemComponent.SetFloatParameter` _returnvalue_3 "Radius" (`self.SpeedBuffRange`))))
              (bind _returnvalue_4 (`self.GetRangeCharacters` (`self.SpeedEndLocation`) (+ (`self.SpeedBuffRange`) 3.0) "EOT_Deffence"))
              (for _array_element _returnvalue_4
                (switch `EObjectType` _controllerobjecttype
                  (:`EOT_Offence`
                    (`XR_Character.TriggerMoveFast` _array_element))
                  (:`EOT_Deffence`
                    (`XR_Character.TriggerMoveSlow` _array_element)))))
            (:`else`)))))
    (:`else`)))

(fn `StunArea`
  (if (`SceneComponent.IsVisible` (`self.StunAreaShowNiagara`))
    (if (`self.CanStun`)
      (set `self.CanStun` false)
      (bind _as_bp_player_controller (`self.As BP Player Controller`)
        (:`then`
          (bind _returnvalue (`Player_Controller.IsGestureWorkable` _as_bp_player_controller))
          (if _returnvalue
            (`SceneComponent.SetVisibility` (`self.StunAreaShowNiagara`) false false)
            (`Player_Controller.SetGestureCoolTime` _as_bp_player_controller)
            (bind _returnvalue_2 (`NiagaraFunctionLibrary.SpawnSystemAtLocation` "/Game/Niagara/NS_StunRangeRing.NS_StunRangeRing" (`self.StunEndLocation`)))
            (`FXSystemComponent.SetFloatParameter` _returnvalue_2 "Radius" (`self.StunRange`))
            (bind _as_bp_player_controller_2 (`self.As BP Player Controller`)
              (:`then`
                (bind _returnvalue_3 (`self.GetRangeCharacters` (`self.StunEndLocation`) (+ (`self.StunRange`) 3.0) (`Player_Controller.controllerObjectType` _as_bp_player_controller_2)))
                (for _array_element _returnvalue_3
                  (`XR_Character.TriggerStun` _array_element)))
              (:`else`))))
        (:`else`)))))

(fn `UserConstructionScript`)