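; Player pawn that turns hand-tracking pose recognition into Grab, Rock, Paper, Scissors and Thumb poses for each hand.
; Each tick it polls both pose recognizers, swaps each hand's material to match and reports the pose to BP_PlayerController.
; Pose action events switch each recognizer's confidence floor between default and activating thresholds, depending on whether a pose is active.
; Right-hand gestures are also polled but trigger nothing, and input actions log encoded poses.
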(event `InputAction|LogLeftHand`
  (params (Key :type "Key Structure"))
  ;[1 1 1] HandPoseLog
  (:`Released`
    (`HandPoseRecognizer.LogEncodedHandPose` (`self.LeftHandPoseRecognizer`))))

(event `RightPoseThresholdChange`
  (params (isDefault :type Boolean))
  ;[1 1 1] HandPoseRecognize Threshold Change
  (if isDefault
    (set `HandPoseRecognizer.DefaultConfidenceFloor` (`self.PoseDefaultThreshold`) (`self.RightHandPose`))
    (else
      (set `HandPoseRecognizer.DefaultConfidenceFloor` (`self.PoseActivatingThreshold`) (`self.RightHandPose`)))))

(event `self.PoseRightAction`
  (params (currentPose :type "Pose Enum" :default "Grab"))
  (if (`|EnumEquality` currentPose)
    (`self.RightPoseThresholdChange` true)
    (else
      (`self.RightPoseThresholdChange` false))))

(event `InputAction|LogRightHand`
  (params (Key :type "Key Structure"))
  ;[1 1 1] HandPoseLog
  (:`Released`
    (`HandPoseRecognizer.LogEncodedHandPose` (`self.RightHandPoseRecognizer`))))

(event `LeftPoseThresholdChange`
  (params (isDefault :type Boolean))
  ;[1 1 1] HandPoseRecognize Threshold Change
  (if isDefault
    (set `HandPoseRecognizer.DefaultConfidenceFloor` (`self.PoseDefaultThreshold`) (`self.LeftHandPose`))
    (else
      (set `HandPoseRecognizer.DefaultConfidenceFloor` (`self.PoseActivatingThreshold`) (`self.LeftHandPose`)))))

(event `self.PoseLeftAction`
  (params (currentPose :type "Pose Enum" :default "Grab"))
  (if (`|EnumEquality` currentPose)
    (`self.LeftPoseThresholdChange` true)
    (else
      (`self.LeftPoseThresholdChange` false))))

(event `self.ReceiveBeginPlay`
  (`|ExecutionSequence`
    (:`then_0`
      (bind _asbp_player_controller (cast `/Game/Blueprints/Controller/BP_PlayerController` (`self.GetController`)))
      (set `self.As BP Player Controller` _asbp_player_controller))
    (:`then_1`
      (`self.RightPoseThresholdChange` true)
      (`self.LeftPoseThresholdChange` true))))

(event `self.ReceiveTick`
  (params (DeltaSeconds :type "Float (single-precision)"))
  (bind (_index _name _duration _error _confidence _returnvalue) (`HandPoseRecognizer.GetRecognizedHandPose` (`self.RightHandPose`)))
  (`self.RightPoseInputCheck` _name _returnvalue)
  (bind (_index_2 _name_2 _duration_2 _error_2 _confidence_2 _returnvalue_2) (`HandPoseRecognizer.GetRecognizedHandPose` (`self.LeftHandPose`)))
  (`self.LeftPoseInputCheck` _name_2 _returnvalue_2)
  (bind (_index_3 _name_3 _gesturedirection _gestureouterduration _gestureinnerduration _returnvalue_3) (`HandGestureRecognizer.GetRecognizedHandGesture` (`self.RightHandGesture`) "Reset"))
  (`self.RightGesture` _name_3 _returnvalue_3))

(fn `Change Hand Color`
  (params (`Material Hand` :type "OculusXRHandComponent Object Reference") (Gesture :type "Pose Enum" :default "Grab"))
  (locals (Material :type "MaterialInterface Object Reference"))
  (switch `Pose` Gesture
    (:`Grab`
      (set `local.Material` (`self.Grab Material`)))
    (:`Rock`
      (set `local.Material` (`self.Rock Material`)))
    (:`scissors`
      (set `local.Material` (`self.Scissor Materail`)))
    (:`Paper`
      (set `local.Material` (`self.Paper Material`)))
    (:`Thumb`
      (set `local.Material` (`self.Thumb Material`)))
    (:`None`
      (set `local.Material` (`self.NULLMaterial`))))
  (`PrimitiveComponent.SetMaterial` (`local.Material Hand`) 0 (`local.Material`)))

(fn `LeftPoseInputCheck`
  (params (PoseName :type String) (bPoseRecognized :type Boolean))
  (locals (RecognizePose :type "Pose Enum" :default "scissors"))
  (if bPoseRecognized
    (switch `string` PoseName
      (:`Default`
        (set `local.RecognizePose` "None" :!label _label))
      (:`Grab`
        (set `local.RecognizePose` "Grab"))
      (:`Scissors`
        (set `local.RecognizePose` "scissors"))
      (:`Rock`
        (set `local.RecognizePose` "Rock"))
      (:`Paper`
        (set `local.RecognizePose` "Paper"))
      (:`Thumb`
        (set `local.RecognizePose` "Thumb")))
    (else
      (goto _label)))
  (`self.Change Hand Color` (`self.LeftHand`) (`local.RecognizePose`))
  (bind _as_bp_player_controller (`self.As BP Player Controller`)
    (:`then`
      (`Player_Controller.UpdateCurrentLeftPose` _as_bp_player_controller (`local.RecognizePose`)))
    (:`else`)))

(fn `RightGesture`
  (params (Selection :type String) (isGestureRecognized :type Boolean))
  (if isGestureRecognized
    (switch `string` Selection)))

(fn `RightPoseInputCheck`
  (params (PoseName :type String) (bPoseRecognized :type Boolean))
  (locals (RecognizePose :type "Pose Enum" :default "None"))
  (if bPoseRecognized
    (switch `string` PoseName
      (:`Default`
        (set `local.RecognizePose` "None" :!label _label))
      (:`Grab`
        (set `local.RecognizePose` "Grab"))
      (:`Scissors`
        (set `local.RecognizePose` "scissors"))
      (:`Rock`
        (set `local.RecognizePose` "Rock"))
      (:`Paper`
        (set `local.RecognizePose` "Paper"))
      (:`Thumb`
        (set `local.RecognizePose` "Thumb")))
    (else
      (goto _label)))
  (`self.Change Hand Color` (`self.RightHand`) (`local.RecognizePose`))
  (bind _as_bp_player_controller (`self.As BP Player Controller`)
    (:`then`
      (`Player_Controller.UpdateCurrentRightPose` _as_bp_player_controller (`local.RecognizePose`)))
    (:`else`)))

(fn `UserConstructionScript`)